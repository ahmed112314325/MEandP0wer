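; BP_Marker is a world marker actor that shows the player's distance to it.
; On BeginPlay it moves itself to its Target location.
; Each Tick it measures the distance to player character 0, converts it to truncated whole meters with an "m" suffix, and passes that text to the Marker component's widget through SetDistanceMessage.
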(event `self.ReceiveBeginPlay`
  (`self.K2_SetActorLocation` (`self.Target`)))

(event `self.ReceiveTick`
  (params (DeltaSeconds :type "Float (single-precision)"))
  (message `/Game/Ui/NavigationInterface.SetDistance` (`WidgetComponent.GetUserWidgetObject` (`self.Marker`)) (`KismetTextLibrary.Conv_StringToText` (`KismetStringLibrary.Concat_StrStr` (`KismetStringLibrary.Conv_IntToString` (`KismetMathLibrary.FTrunc` (/ (`KismetMathLibrary.Vector_Distance` (`self.K2_GetActorLocation`) (`self.K2_GetActorLocation` (`GameplayStatics.GetPlayerCharacter` 0))) 100.0))) "m"))))

(fn `UserConstructionScript`)